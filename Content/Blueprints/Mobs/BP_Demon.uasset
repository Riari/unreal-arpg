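; BP_Demon is a mob Blueprint that shows an enemy info widget while the cursor hovers over the living demon.
; BeginPlay creates the BP_EnemyInfo widget with the mob's name and health ratio from HealthComponent.
; Cursor-over events add it to and remove it from the viewport.
; Tick refreshes the health percentage every frame and removes the widget whenever the demon is not alive.
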(event `self.ReceiveBeginPlay`
  (bind _healthcomponent (`self.HealthComponent`))
  (bind _returnvalue (`|CreateWidget` "/Game/UI/HUD/BP_EnemyInfo.BP_EnemyInfo_C"))
  (set `/Game/UI/HUD/BP_EnemyInfo.Name` (`self.MobName`) _returnvalue)
  (set `/Game/UI/HUD/BP_EnemyInfo.HealthPercentage` (`KismetMathLibrary.SafeDivide` (`HealthComponent.Health` _healthcomponent) (`HealthComponent.MaxHealth` _healthcomponent)) _returnvalue))

(event `self.ReceiveActorBeginCursorOver`
  (if (`self.bIsAlive`)
    (`UserWidget.AddToViewport` (stale `self.ReceiveBeginPlay` _returnvalue) 0)))

(event `self.ReceiveActorEndCursorOver`
  (`Widget.RemoveFromParent` (stale `self.ReceiveBeginPlay` _returnvalue)))

(event `self.ReceiveTick`
  (params (DeltaSeconds :type "Float (single-precision)"))
  (bind _healthcomponent (`self.HealthComponent`))
  (set `/Game/UI/HUD/BP_EnemyInfo.HealthPercentage` (`KismetMathLibrary.SafeDivide` (`HealthComponent.Health` _healthcomponent) (`HealthComponent.MaxHealth` _healthcomponent)) (stale `self.ReceiveBeginPlay` _returnvalue))
  (if (not (`self.bIsAlive`))
    (`Widget.RemoveFromParent` (stale `self.ReceiveBeginPlay` _returnvalue))))

(fn `UserConstructionScript`)